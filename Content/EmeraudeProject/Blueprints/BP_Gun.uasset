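; BP_Gun is a Russian roulette style gun with one deadly bullet hidden in a random chamber.
; On BeginPlay it picks the dead-bullet slot at random within its capacity.
; TryShoot returns true when the current slot matches that slot, otherwise it advances the slot and returns false.
; Both steps print debug text in French, which reveals the capacity, deadly slot and current slot.
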(event EventBeginPlay
  (bind _output_get (Variables|GunSettings|SetslotDeadBullet (Math|Random|RandomInteger (Variables|GunSettings|Getcapacity))))
  (Development|PrintText (Utilities|Text|FormatText "La capacité du gun : {capacity} 
Le slot de la mort : {slot}" (Variables|GunSettings|Getcapacity) _output_get) true true "(R=1.000000,G=0.280420,B=0.545578,A=1.000000)" 99999999.0))

(fn ConstructionScript)

(fn TryShoot()
  (Development|PrintText (Utilities|Text|FormatText "Le slot actuel : {currentSlot}" (Variables|GunSettings|GetshootingSlot)) true true "(R=0.000000,G=0.410243,B=1.000000,A=1.000000)")
  (if (== (Variables|GunSettings|GetshootingSlot) (Variables|GunSettings|GetslotDeadBullet))
    (return true)
    (else
      (Math|Integer|IncrementInt (Variables|GunSettings|GetshootingSlot)
        (:%20%20
          (return false))))))