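; Lobby game mode that tracks connected players and can send the server to Level_GunShoot.
; On each login it reads the session settings and adds the controller to Controllers while the list count is at or below NumConnections.
; Once the count exceeds that number, a further login triggers server travel instead of being added.
; It prints the current and maximum counts after a successful settings read, and removes controllers on logout.
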(event EventBeginPlay)

(event EventTick
  (params (DeltaSeconds :type Float%20%28single-precision%29)))

(event EventPostLogin
  (params (NewPlayer :type Player%20Controller%20Object%20Reference))
  (bind _numconnections (Class|AdvancedSessionsLibrary|GetSessionSettings)
    (:OnSuccess
      (if (<= (Utilities|Array|Length (Variables|Default|GetControllers)) _numconnections)
        (Utilities|Array|AddUnique (Variables|Default|GetControllers) NewPlayer)
        (else
          (Development|ExecuteConsoleCommand "serverTravel Level_GunShoot" 0)))
      (Development|PrintText (Utilities|Text|FormatText "nbr current client : {nbrCurrentClient} 
nbr max client : {nbrMaxClient}" (Utilities|Array|Length (Variables|Default|GetControllers)) _numconnections)))))

(event EventOnLogout
  (params (ExitingController :type Controller%20Object%20Reference))
  (bind _asplayer_controller (Utilities|Casting|CastToPlayerController ExitingController))
  (Utilities|Array|RemoveItem (Variables|Default|GetControllers) _asplayer_controller))

(fn ConstructionScript)